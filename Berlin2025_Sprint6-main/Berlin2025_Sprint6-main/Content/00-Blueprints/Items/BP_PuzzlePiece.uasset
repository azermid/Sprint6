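; BP_PuzzlePiece is an item Blueprint for one of sixteen pieces of a puzzle, identified by its Id.
; On BeginPlay, a switch on Id picks the piece's Icon image and its X/Y offset in a four-by-four grid.
; Shared branches set each row's Y before the Puzzle mesh takes the Id-indexed entry from NewVar and moves to that relative position.
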(event `self.ReceiveBeginPlay`
  (switch `int` (`self.Id`)
    (:`0`
      (set `self.Icon` "/Game/00-Blueprints/Items/IconPuzzle/Capture_d_écran_2026-05-20_041408-removebg-preview.Capture_d_écran_2026-05-20_041408-removebg-preview")
      (set `self.XValue` 15.0)
      (set `self.YValue` 15.0 :!label _label))
    (:`1`
      (set `self.Icon` "/Game/00-Blueprints/Items/IconPuzzle/Capture_d_écran_2026-05-20_041430-removebg-preview.Capture_d_écran_2026-05-20_041430-removebg-preview")
      (set `self.XValue` 5.0)
      (goto _label))
    (:`2`
      (set `self.Icon` "/Game/00-Blueprints/Items/IconPuzzle/Capture_d_écran_2026-05-20_041458-removebg-preview.Capture_d_écran_2026-05-20_041458-removebg-preview")
      (set `self.XValue` -5.0)
      (goto _label))
    (:`3`
      (set `self.Icon` "/Game/00-Blueprints/Items/IconPuzzle/Capture_d_écran_2026-05-20_041518-removebg-preview.Capture_d_écran_2026-05-20_041518-removebg-preview")
      (set `self.XValue` -16.0)
      (goto _label))
    (:`4`
      (set `self.Icon` "/Game/00-Blueprints/Items/IconPuzzle/Capture_d_écran_2026-05-20_041543-removebg-preview.Capture_d_écran_2026-05-20_041543-removebg-preview")
      (set `self.XValue` 15.0)
      (set `self.YValue` 5.0 :!label _label_2))
    (:`5`
      (set `self.Icon` "/Game/00-Blueprints/Items/IconPuzzle/image_2026-05-20_152406795-removebg-preview.image_2026-05-20_152406795-removebg-preview")
      (set `self.XValue` 5.0)
      (goto _label_2))
    (:`6`
      (set `self.Icon` "/Game/00-Blueprints/Items/IconPuzzle/Capture_d_écran_2026-05-20_041607-removebg-preview.Capture_d_écran_2026-05-20_041607-removebg-preview")
      (set `self.XValue` -5.0)
      (goto _label_2))
    (:`7`
      (set `self.Icon` "/Game/00-Blueprints/Items/IconPuzzle/Capture_d_écran_2026-05-20_041623-removebg-preview.Capture_d_écran_2026-05-20_041623-removebg-preview")
      (set `self.XValue` -15.0)
      (goto _label_2))
    (:`8`
      (set `self.Icon` "/Game/00-Blueprints/Items/IconPuzzle/Capture_d_écran_2026-05-20_041638-removebg-preview.Capture_d_écran_2026-05-20_041638-removebg-preview")
      (set `self.XValue` 15.0)
      (set `self.YValue` -5.0 :!label _label_3))
    (:`9`
      (set `self.Icon` "/Game/00-Blueprints/Items/IconPuzzle/Capture_d_écran_2026-05-20_041656-removebg-preview.Capture_d_écran_2026-05-20_041656-removebg-preview")
      (set `self.XValue` 5.0)
      (goto _label_3))
    (:`10`
      (set `self.Icon` "/Game/00-Blueprints/Items/IconPuzzle/Capture_d_écran_2026-05-20_041714-removebg-preview.Capture_d_écran_2026-05-20_041714-removebg-preview")
      (set `self.XValue` -5.0)
      (goto _label_3))
    (:`11`
      (set `self.Icon` "/Game/00-Blueprints/Items/IconPuzzle/Capture_d_écran_2026-05-20_041730-removebg-preview.Capture_d_écran_2026-05-20_041730-removebg-preview")
      (set `self.XValue` -15.0)
      (goto _label_3))
    (:`12`
      (set `self.Icon` "/Game/00-Blueprints/Items/IconPuzzle/Capture_d_écran_2026-05-20_041746-removebg-preview.Capture_d_écran_2026-05-20_041746-removebg-preview")
      (set `self.XValue` 15.0)
      (set `self.YValue` -15.0 :!label _label_4))
    (:`13`
      (set `self.Icon` "/Game/00-Blueprints/Items/IconPuzzle/Capture_d_écran_2026-05-20_041802-removebg-preview.Capture_d_écran_2026-05-20_041802-removebg-preview")
      (set `self.XValue` 5.0)
      (goto _label_4))
    (:`14`
      (set `self.Icon` "/Game/00-Blueprints/Items/IconPuzzle/Capture_d_écran_2026-05-20_041817-removebg-preview.Capture_d_écran_2026-05-20_041817-removebg-preview")
      (set `self.XValue` -5.0)
      (goto _label_4))
    (:`15`
      (set `self.Icon` "/Game/00-Blueprints/Items/IconPuzzle/Capture_d_écran_2026-05-20_041832-removebg-preview.Capture_d_écran_2026-05-20_041832-removebg-preview")
      (set `self.XValue` -15.0)
      (goto _label_4)))
  (`StaticMeshComponent.SetStaticMesh` (`self.Puzzle`) (`|GetArrayItem` (`self.NewVar`) (`self.Id`)))
  (`SceneComponent.K2_SetRelativeLocation` (`self.Puzzle`) (`KismetMathLibrary.MakeVector` (`self.XValue`) (`self.YValue`)) false false))

(fn `UserConstructionScript`)