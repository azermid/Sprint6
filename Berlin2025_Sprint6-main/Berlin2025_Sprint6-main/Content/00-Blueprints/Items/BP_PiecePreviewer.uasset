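; Piece previewer actor that provides live preview images of sixteen pieces as materials.
; Each scene capture is restricted to its own piece mesh, while each render target feeds a dynamic M_PiecePreview material, retrieved by one-based number through GetRenderMatN.
; RotatePiece smoothly turns a chosen piece to a target rotation with RInterpTo on a looping timer, ignoring new requests while a turn is running.
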(event `self.ReceiveBeginPlay`
  (set `self.ArrayMesh` (`|MakeArray` (`self.Piece`) (`self.Piece1`) (`self.Piece2`) (`self.Piece3`) (`self.Piece4`) (`self.Piece5`) (`self.Piece6`) (`self.Piece7`) (`self.Piece8`) (`self.Piece9`) (`self.Piece10`) (`self.Piece11`) (`self.Piece12`) (`self.Piece13`) (`self.Piece14`) (`self.Piece15`)))
  (set `self.SceneCaputeArray` (`|MakeArray` (`self.SceneCaptureComponent2D`) (`self.SceneCaptureComponent2D1`) (`self.SceneCaptureComponent2D2`) (`self.SceneCaptureComponent2D3`) (`self.SceneCaptureComponent2D4`) (`self.SceneCaptureComponent2D5`) (`self.SceneCaptureComponent2D6`) (`self.SceneCaptureComponent2D7`) (`self.SceneCaptureComponent2D8`) (`self.SceneCaptureComponent2D9`) (`self.SceneCaptureComponent2D10`) (`self.SceneCaptureComponent2D11`) (`self.SceneCaptureComponent2D12`) (`self.SceneCaptureComponent2D13`) (`self.SceneCaptureComponent2D14`) (`self.SceneCaptureComponent2D15`)))
  (bind _output_get (set `self.renderTextureArray` (`|MakeArray` "/Game/00-Blueprints/Items/RenderPiece/RT_PiecePreviewN1.RT_PiecePreviewN1" "/Game/00-Blueprints/Items/RenderPiece/RT_PiecePreviewN2.RT_PiecePreviewN2" "/Game/00-Blueprints/Items/RenderPiece/RT_PiecePreviewN3.RT_PiecePreviewN3" "/Game/00-Blueprints/Items/RenderPiece/RT_PiecePreviewN4.RT_PiecePreviewN4" "/Game/00-Blueprints/Items/RenderPiece/RT_PiecePreviewN5.RT_PiecePreviewN5" "/Game/00-Blueprints/Items/RenderPiece/RT_PiecePreviewN6.RT_PiecePreviewN6" "/Game/00-Blueprints/Items/RenderPiece/RT_PiecePreviewN7.RT_PiecePreviewN7" "/Game/00-Blueprints/Items/RenderPiece/RT_PiecePreviewN8.RT_PiecePreviewN8" "/Game/00-Blueprints/Items/RenderPiece/RT_PiecePreviewN9.RT_PiecePreviewN9" "/Game/00-Blueprints/Items/RenderPiece/RT_PiecePreviewN10.RT_PiecePreviewN10" "/Game/00-Blueprints/Items/RenderPiece/RT_PiecePreviewN11.RT_PiecePreviewN11" "/Game/00-Blueprints/Items/RenderPiece/RT_PiecePreviewN12.RT_PiecePreviewN12" "/Game/00-Blueprints/Items/RenderPiece/RT_PiecePreviewN13.RT_PiecePreviewN13" "/Game/00-Blueprints/Items/RenderPiece/RT_PiecePreviewN14.RT_PiecePreviewN14" "/Game/00-Blueprints/Items/RenderPiece/RT_PiecePreviewN15.RT_PiecePreviewN15" "/Game/00-Blueprints/Items/RenderPiece/RT_PiecePreviewN16.RT_PiecePreviewN16" :!type "Texture Object Reference")))
  (for _array_element _output_get
    (bind _returnvalue (`KismetMaterialLibrary.CreateDynamicMaterialInstance` "/Game/00-Blueprints/Items/RenderPiece/M_PiecePreview.M_PiecePreview"))
    (`MaterialInstanceDynamic.SetTextureParameterValue` _returnvalue "PieceTexture" _array_element)
    (`KismetArrayLibrary.Array_AddUnique` (`self.MateriauxArray`) _returnvalue))
  (for (_array_element_2 _array_index) (`self.SceneCaputeArray`)
    (`SceneCaptureComponent.ShowOnlyComponent` _array_element_2 (`|GetArrayItem` (`self.ArrayMesh`) _array_index))))

(event `RotatePiece?`
  (params (NewParam :type Integer) (NewParam2 :type "Rotator Structure"))
  (if (not (`self.IsTruning`))
    (set `self.CurrentPiece` NewParam)
    (set `self.TargetRot` NewParam2)
    (bind _returnvalue (`KismetSystemLibrary.K2_SetTimerDelegate` (delegate `CustomEvent`) 0.01 true))
    (set `self.RotationTimerHandler` _returnvalue)))

(event `CustomEvent`
  (bind _output (`|GetArrayItem` (`self.ArrayMesh`) (`self.CurrentPiece`)))
  (set `self.IsTruning` true)
  (`SceneComponent.K2_SetWorldRotation` _output (`KismetMathLibrary.RInterpTo` (`SceneComponent.K2_GetComponentRotation` _output) (`self.TargetRot`) (`GameplayStatics.GetWorldDeltaSeconds`) 15.0) false false)
  (if (== (`self.TargetRot`) (`SceneComponent.K2_GetComponentRotation` _output))
    (set `self.IsTruning` false)
    (`KismetSystemLibrary.K2_ClearAndInvalidateTimerHandle` (`self.RotationTimerHandler`))))

(fn `GetRenderMatN?`
  (params (A :type Integer))
  (returns (Output1 :type "MaterialInstanceDynamic Object Reference"))
  (return (`|GetArrayItem` (`self.MateriauxArray`) (- A 1))))

(fn `UserConstructionScript`)