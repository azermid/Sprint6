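; Crystal pedestal for an enigma that accepts one crystal and shows whether its type matches the pedestal's FeelingType.
; On sphere overlap it force-ungrabs the player, snaps the crystal into place, plays a sound and turns the light green or red.
; Correct placements increment a counter on BP_FPSPlayer, and reaching three calls EnigmaIsValid.
; Removing the crystal resets the light and slot, decrementing the counter if it matched.
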(event `self.ReceiveBeginPlay`
  (bind _asbp_fpsplayer (cast `/Game/00-Blueprints/Player/BP_FPSPlayer` (`GameplayStatics.GetPlayerCharacter` 0)))
  (set `self.PlayerRef` _asbp_fpsplayer))

(event `self.Sphere.OnComponentBeginOverlap`
  (params (OverlappedComponent :type "PrimitiveComponent Object Reference") (OtherActor :type "Actor Object Reference") (OtherComp :type "PrimitiveComponent Object Reference") (OtherBodyIndex :type Integer) (bFromSweep :type Boolean) (SweepResult :type "HitResult Structure (by ref)"))
  (if (not (`self.AlreadyHasACrystalOn`))
    (`/Engine/EditorBlueprintResources/StandardMacros.IsValid` (`self.CrystalOnPiedestral`)
      (:`Is Not Valid`
        (bind _asbp_item_crystals (cast `/Game/00-Blueprints/Items/BP_Item_Crystals` OtherActor))
        (set `self.CrystalOnPiedestral` _asbp_item_crystals)
        (`/Game/00-Blueprints/Player/BP_FPSPlayer.ForceUngrab` (`self.PlayerRef`))
        (`self.K2_AttachToComponent` _asbp_item_crystals (`self.CrystalPos`) "None" "SnapToTarget" "SnapToTarget" "KeepWorld" true)
        (`GameplayStatics.PlaySoundAtLocation` "/Game/02-Musics_SFX/putting-glass-object-on-table-sound-effect-mfsl-no-copyright_ygTLcnQ5.putting-glass-object-on-table-sound-effect-mfsl-no-copyright_ygTLcnQ5" (`SceneComponent.K2_GetComponentLocation` (`self.Sphere`)) (struct) 2.0 1.0 0.0 "/Game/02-Musics_SFX/SA_Crystals.SA_Crystals" null null null)
        (if (`|EnumEquality` (`/Game/00-Blueprints/Items/BP_Item_Crystals.CrystalType` _asbp_item_crystals) (`self.FeelingType`))
          (`self.GoodCrystal`)
          (`KismetSystemLibrary.PrintString` "GoodCrystal")
          (bind _result (`/Engine/EditorBlueprintResources/StandardMacros.IncrementInt` (`/Game/00-Blueprints/Player/BP_FPSPlayer.FirstEnigma_TotalValid` (`self.PlayerRef`)))
            (:`  `
              (`KismetSystemLibrary.PrintString` (`KismetStringLibrary.Concat_StrStr` "test: " (`KismetStringLibrary.Conv_IntToString` _result)))
              (`self.CheckIfEnigmaIsOver`)))
          (else
            (`self.WrongCrystal`)
            (`KismetSystemLibrary.PrintString` "WrongCrystal")))
        (set `self.AlreadyHasACrystalOn` true)))))

(event `self.Sphere.OnComponentEndOverlap`
  (params (OverlappedComponent :type "PrimitiveComponent Object Reference") (OtherActor :type "Actor Object Reference") (OtherComp :type "PrimitiveComponent Object Reference") (OtherBodyIndex :type Integer))
  (bind _asbp_item_crystals (cast `/Game/00-Blueprints/Items/BP_Item_Crystals` OtherActor))
  (if (== (`self.CrystalOnPiedestral`) _asbp_item_crystals)
    (if (`|EnumEquality` (`/Game/00-Blueprints/Items/BP_Item_Crystals.CrystalType` _asbp_item_crystals) (`self.FeelingType`))
      (`/Engine/EditorBlueprintResources/StandardMacros.DecrementInt` (`/Game/00-Blueprints/Player/BP_FPSPlayer.FirstEnigma_TotalValid` (`self.PlayerRef`))
        (:`  `
          _)))
    (`LightComponent.SetLightColor` (`self.LightComponent0`) (struct :`R` 1.0 :`G` 1.0 :`B` 1.0 :`A` 1.0) true)
    (set `self.AlreadyHasACrystalOn` false)
    (set `self.CrystalOnPiedestral` null)))

(event `WrongCrystal`
  (`LightComponent.SetLightColor` (`self.LightComponent0`) (struct :`R` 1.0 :`G` 0.102599 :`A` 1.0) true))

(event `GoodCrystal`
  (`LightComponent.SetLightColor` (`self.LightComponent0`) (struct :`G` 1.0 :`B` 0.097419 :`A` 1.0) true))

(event `CheckIfEnigmaIsOver`
  (if (== (`/Game/00-Blueprints/Player/BP_FPSPlayer.FirstEnigma_TotalValid` (`self.PlayerRef`)) 3)
    (`self.EnigmaIsValid`)
    (`KismetSystemLibrary.PrintString` "ENIGMA END" true true (struct :`R` 1.0 :`G` 0.10567 :`A` 1.0))))

(fn `UserConstructionScript`
  (`parent.UserConstructionScript`))