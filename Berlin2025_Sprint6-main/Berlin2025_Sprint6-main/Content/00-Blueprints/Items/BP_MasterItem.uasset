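; BP_MasterItem is a base item Blueprint that shows a decal outline while it is being looked at as an interactable.
; StartLookatInteractables and StopLookatInteractables toggle the DecalOutline's visibility through EnableOutline and DisableOutline.
; BeginPlay hides the outline and prints a debug message.
; The construction script applies DecalSize and ShapeScale as world scales to the outline decal and the SMShape component.
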(event `self.ReceiveBeginPlay`
  (`self.DisableOutline`)
  (`KismetSystemLibrary.PrintText` "Hello"))

(event `EnableOutline`
  (`SceneComponent.SetHiddenInGame` (`self.Decal_Outline`) false true))

(event `DisableOutline`
  (`SceneComponent.SetHiddenInGame` (`self.Decal_Outline`) true false))

(event `/Game/00-Blueprints/Interfaces/BPI_Interactables.StartLookAtInteractables`
  (`self.EnableOutline`))

(event `/Game/00-Blueprints/Interfaces/BPI_Interactables.StopLookAtInteractables`
  (`self.DisableOutline`))

(fn `UserConstructionScript`
  (`SceneComponent.SetWorldScale3D` (`self.Decal_Outline`) (`self.DecalSize`))
  (`SceneComponent.SetWorldScale3D` (`self.SM_Shape`) (`self.ShapeScale`)))