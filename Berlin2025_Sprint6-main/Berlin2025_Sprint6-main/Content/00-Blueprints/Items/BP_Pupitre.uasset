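; Puzzle lectern (pupitre) where the player arranges BP_PuzzlePiece actors on a sixteen-slot board through WBP_PupitreMainHud.
; InitPupitre picks random world pieces and slots, then pre-fills them through a temporary widget, making those pieces non-takeable.
; Action opens a fresh HUD and reloads the layout from PieceArray, which Saved rebuilds from the slots.
; CheckWin compares piece Ids to slot indices, then forces the player off and fires PuzzleSolved.
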(event `InitCase`
  (params (NewParam :type "/Game/00-Blueprints/Widgets/WBP_PupitreMainHud Object Reference"))
  (for (_array_element _array_index) (`self.IndexbusyArray`)
    (bind _output (`|GetArrayItem` (`self.Piece_Array`) _array_index))
    (`SceneComponent.SetVisibility` (`/Game/00-Blueprints/Items/BP_PuzzlePiece.DefaultSceneRoot` _output) true true)
    (bind _output_2 (`|GetArrayItem` (`/Game/00-Blueprints/Widgets/WBP_PupitreMainHud.ArrayCase` NewParam) _array_element))
    (set `/Game/00-Blueprints/Widgets/CaseGrid.Puzzle Piece` _output _output_2)
    (set `/Game/00-Blueprints/Items/BP_PuzzlePiece.IsTakeAble` false _output)
    (`/Game/00-Blueprints/Widgets/CaseGrid.SetNewPiece` _output_2))
  (`Widget.RemoveFromParent` NewParam))

(event `InitPupitre`
  (bind _output (`|GetArrayItem` (`self.IndexArray`) (`.OutIndex` (`KismetArrayLibrary.Array_Random` (`self.IndexArray`)))))
  (bind _outactors (`GameplayStatics.GetAllActorsOfClass` "/Game/00-Blueprints/Items/BP_PuzzlePiece.BP_PuzzlePiece_C"))
  (for _ (range 12)
    (`KismetArrayLibrary.Array_AddUnique` (`self.IndexbusyArray`) _output)
    (`KismetArrayLibrary.Array_RemoveItem` (`self.IndexArray`) _output)
    (bind _output_2 (`|GetArrayItem` _outactors (`.OutIndex` (`KismetArrayLibrary.Array_Random` _outactors))))
    (`SceneComponent.SetHiddenInGame` (`/Game/00-Blueprints/Items/BP_PuzzlePiece.DefaultSceneRoot` _output_2) true true)
    (`KismetArrayLibrary.Array_AddUnique` (`self.Piece_Array`) _output_2)
    (`KismetArrayLibrary.Array_RemoveItem` _outactors _output_2))
  (bind _asbp_fpsplayer (cast `/Game/00-Blueprints/Player/BP_FPSPlayer` (`GameplayStatics.GetPlayerPawn` 0)))
  (bind _returnvalue (`|CreateWidget` "/Game/00-Blueprints/Widgets/WBP_PupitreMainHud.WBP_PupitreMainHud_C" null _asbp_fpsplayer self))
  (`self.InitCase` _returnvalue))

(event `self.ReceiveBeginPlay`
  (set `self.PointArray` (`|MakeArray` (`self.POint1`) (`self.Point2`) (`self.Point3`) (`self.Point4`) (`self.Point5`) (`self.Point6`) (`self.Point7`) (`self.Point8`) (`self.Point9`) (`self.Point10`) (`self.Point11`) (`self.Point12`) (`self.Point13`) (`self.Point14`) (`self.Point15`) (`self.Point16`)))
  (set `self.ArrayHavePiece` (`|MakeArray` false false false false false false false false false false false false false false false false))
  (set `self.IndexArray` (`|MakeArray` 0 1 2 3 4 5 6 7 8 9 10 11 12 13 14 15))
  (bind _returnvalue (`GameplayStatics.GetActorOfClass` "/Game/00-Blueprints/Player/BP_FPSPlayer.BP_FPSPlayer_C"))
  (set `self.Player` _returnvalue))

(event `Action`
  (params (Player :type "/Game/00-Blueprints/Player/BP_FPSPlayer Object Reference"))
  (bind _returnvalue (`|CreateWidget` "/Game/00-Blueprints/Widgets/WBP_PupitreMainHud.WBP_PupitreMainHud_C" null Player self))
  (set `self.HUD` _returnvalue)
  (`KismetSystemLibrary.Delay` 0.5)
  (`self.LoadSave`)
  (`UserWidget.AddToViewport` (`self.HUD`) 0)
  (set `PlayerController.bShowMouseCursor` true (`GameplayStatics.GetPlayerController` 0))
  (add `/Game/00-Blueprints/Widgets/WBP_PupitreMainHud.CheckWin` (`self.HUD`) (delegate `CheckWin`)))

(event `CheckWin`
  (`self.CheckWinFunct`))

(event `Saved`
  (`KismetArrayLibrary.Array_Clear` (`self.Piece_Array`))
  (for _array_element (`/Game/00-Blueprints/Widgets/WBP_PupitreMainHud.ArrayCase` (`self.HUD`))
    (`KismetArrayLibrary.Array_Add` (`self.Piece_Array`) (`/Game/00-Blueprints/Widgets/CaseGrid.Puzzle Piece` _array_element))))

(event `LoadSave`
  (`/Game/00-Blueprints/Widgets/WBP_PupitreMainHud.LoadSaved` (`self.HUD`) (`self.Piece_Array`)))

(fn `CheckWinFunct`
  (locals (IsWinning :type Boolean :default true))
  (if (not (`self.IsFinished`))
    (for (_array_element _array_index) (`/Game/00-Blueprints/Widgets/WBP_PupitreMainHud.ArrayCase` (`self.HUD`))
      (bind _puzzle_piece (`/Game/00-Blueprints/Widgets/CaseGrid.Puzzle Piece` _array_element))
      (`/Engine/EditorBlueprintResources/StandardMacros.IsValid` _puzzle_piece
        (:`Is Valid`
          (if (not (== (`/Game/00-Blueprints/Items/BP_PuzzlePiece.Id` _puzzle_piece) _array_index))
            (set `local.IsWinning` false)))
        (:`Is Not Valid`
          (set `local.IsWinning` false))))
    (if (`local.IsWinning`)
      (`/Game/00-Blueprints/Player/BP_FPSPlayer.ForceUnPupitre` (`self.Player`))
      (`self.PuzzleSolved`)
      (set `self.IsFinished` true))))

(fn `GetClosestPoint`
  (params (NewParam :type "Vector Structure"))
  (returns (NewParam2 :type "Transform Structure") (`Array Element` :type "SceneComponent Object Reference"))
  (locals (Closesed :type "Vector Structure" :default (1000.0 1000.0 10000.0)) (ClosesedTransfo :type "Transform Structure") (Point :type "SceneComponent Object Reference"))
  (for _array_element (`self.PointArray`)
    (bind _returnvalue (`SceneComponent.K2_GetComponentLocation` _array_element))
    (if (< (`KismetMathLibrary.Vector_Distance` NewParam _returnvalue) (`KismetMathLibrary.Vector_Distance` NewParam (`local.Closesed`)))
      (set `local.Closesed` _returnvalue)
      (set `local.ClosesedTransfo` (`SceneComponent.K2_GetComponentToWorld` _array_element))
      (set `local.Point` _array_element)))
  (return (`local.ClosesedTransfo`) (`local.Point`)))

(fn `UserConstructionScript`)